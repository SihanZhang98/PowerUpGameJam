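; BP_Planet is a solar system planet actor that can be clicked to focus and dragged to rotate.
; Clicking the planet or cloud mesh broadcasts OnPlanetFocus with itself and starts dragging, and releasing stops it.
; While dragging, Mouse2D input scaled by InteractSensitivity drives roll and pitch, combined with the current rotation.
; Two helper functions toggle IsViewFocused on every entry in PlanetCharacters to make them hoverable or not.
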(event OnClicked(Planet1-repackaged_Clouds_1)
  (params (TouchedComponent :type Primitive%20Component%20Object%20Reference) (ButtonPressed :type Key%20Structure :default "None"))
  (Variables|Default|SetisDragging true)
  (Default|CallOnPlanetFocus self))

(event OnClicked(Planet1-repackaged_Planet_1_001)
  (params (TouchedComponent :type Primitive%20Component%20Object%20Reference) (ButtonPressed :type Key%20Structure :default "None"))
  (Variables|Default|SetisDragging true)
  (Default|CallOnPlanetFocus self))

(event OnReleased(Planet1-repackaged_Planet_1_001)
  (params (TouchedComponent :type Primitive%20Component%20Object%20Reference) (ButtonReleased :type Key%20Structure :default "None"))
  (Variables|Default|SetisDragging false))

(event OnReleased(Planet1-repackaged_Clouds_1)
  (params (TouchedComponent :type Primitive%20Component%20Object%20Reference) (ButtonReleased :type Key%20Structure :default "None"))
  (Variables|Default|SetisDragging false))

(event Collision|EventActorBeginOverlap
  (params (OtherActor :type Actor%20Object%20Reference)))

(event EventTick
  (params (DeltaSeconds :type Float%20%28single-precision%29)))

(event Input|MouseEvents|Mouse2D
  (params (AxisValue :type Vector :default "0, 0, 0"))
  (bind _interactsensitivity (Variables|Default|GetInteractSensitivity))
  (bind _returnvalue (* AxisValue _interactsensitivity))
  (bind (_x _y) (Math|Vector|BreakVector _returnvalue))
  (if (Variables|Default|GetisDragging)
    (Transformation|SetActorRotation (Math|Rotator|CombineRotators (Transformation|GetActorRotation) (Math|Rotator|MakeRotator _x _y 0.0)))))

(fn ConstructionScript)

(fn MakePlanetCharsHoverable
  (for _array_element (Variables|Default|GetPlanetCharacters)
    (Variables|/Game/Blueprints/BP_PlanetCharacter.BP_PlanetCharacter_C|SetisViewFocused _array_element true)))

(fn MakePlanetCharsUnhoverable
  (for _array_element (Variables|Default|GetPlanetCharacters)
    (Variables|/Game/Blueprints/BP_PlanetCharacter.BP_PlanetCharacter_C|SetisViewFocused _array_element false)))