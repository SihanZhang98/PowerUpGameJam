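; Solar system manager that orbits planets and moves the player pawn between system view and planet view.
; Tick circles all planets at a shared radius around their averaged starting position, using per-planet angles.
; A planet focus event pauses orbiting, lerps the pawn toward that planet via Timeline, then enables its input and shows back, fire and outcome widgets.
; The back button resumes orbiting, returns the pawn and removes widgets.
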(event Custom|OnPlanetFocus
  (params (viewPlanet :type BP%20Planet%20Object%20Reference))
  (if (not (Utilities|IsValid (Variables|Default|GetcurrPlanetFocused)))
    (Variables|Default|SetisOrbiting false)
    (bind _output_get (Variables|Default|SetcurrPlanetFocused viewPlanet))
    (CallFunction|SetVectorsforPlanetView (Variables|/Game/SolarSystem/BP_Planet.BP_Planet_C|GetCameraDistanceAway _output_get))
    (bind (_direction _movement _rotation) (Timeline|Timeline PlayFromStart)
      (:Update
        (CallFunction|MovePlayertoNewView _movement _rotation))
      (:Finished
        (Input|EnableInput _output_get (Variables|Default|GetPlayerCtrl))
        (Utilities|FlowControl|Sequence
          (:then_0
            (bind _returnvalue (UserInterface|CreateWidget "/Game/SolarSystem/Widgets/W_BackToSystem.W_BackToSystem_C" (Variables|Default|GetPlayerCtrl)))
            (bind _output_get_2 (Variables|Default|SetBackToSystemWidget _returnvalue))
            (UserInterface|Viewport|AddtoViewport _output_get_2 0)
            (EventDispatchers|BindEventtoOnClickedBackBtn _returnvalue (EventDispatchers|CreateEvent :!event Custom|OnSystemView)))
          (:then_1
            (bind _returnvalue_2 (UserInterface|CreateWidget "/Game/SolarSystem/Widgets/UI_FireBtn_Grayed.UI_FireBtn_Grayed_C" (Variables|Default|GetPlayerCtrl)))
            (bind _output_get_3 (Variables|Default|SetFireBtn _returnvalue_2))
            (UserInterface|Viewport|AddtoViewport _returnvalue_2 0))
          (:then_2
            (if (Variables|/Game/SolarSystem/BP_Planet.BP_Planet_C|GethasOutcome (Variables|Default|GetcurrPlanetFocused))
              (bind _returnvalue_3 (UserInterface|CreateWidget "/Game/Outcomes/W_ShowOutcome.W_ShowOutcome_C" (Variables|Default|GetPlayerCtrl)))
              (UserInterface|Viewport|AddtoViewport _returnvalue_3 0)
              (Rendering|Components|TextRender|SetText (Variables|/Game/Outcomes/W_ShowOutcome.W_ShowOutcome_C|GetOutcomeText _returnvalue_3) (Variables|/Game/SolarSystem/BP_Planet.BP_Planet_C|GetcurrOutcomeTxt (Variables|Default|GetcurrPlanetFocused))))))))))

(event Custom|OnSystemView
  (Variables|/Game/SolarSystem/BP_Planet.BP_Planet_C|SetisPlanetView (Variables|Default|GetcurrPlanetFocused) false)
  (CallFunction|SetVectorsforSystemView)
  (Variables|Default|SetisOrbiting true)
  (Widget|RemovefromParent (Variables|Default|GetBackToSystemWidget))
  (if (Variables|/Game/SolarSystem/BP_Planet.BP_Planet_C|GethasOutcome (Variables|Default|GetcurrPlanetFocused))
    (bind _foundwidgets (Widget|GetAllWidgetsOfClass "/Game/Outcomes/W_ShowOutcome.W_ShowOutcome_C" true))
    (for _array_element _foundwidgets
      (Widget|RemovefromParent _array_element)
      (Variables|Default|SetcurrPlanetFocused 0)
      (bind (_direction _movement _rotation) (Timeline|Timeline_0 PlayFromStart)
        (:Update
          (CallFunction|MovePlayertoNewView _movement _rotation))
        (:Finished
          (Utilities|FlowControl|Sequence
            (:then_0
              (bind _foundwidgets_2 (Widget|GetAllWidgetsOfClass "/Game/SolarSystem/Widgets/UI_FireBtn.UI_FireBtn_C" true))
              (for _array_element_2 _foundwidgets_2
                (Widget|RemovefromParent _array_element_2)))
            (:then_1
              (bind _foundwidgets_3 (Widget|GetAllWidgetsOfClass "/Game/SolarSystem/Widgets/UI_FireBtn_Grayed.UI_FireBtn_Grayed_C" true))
              (for _array_element_3 _foundwidgets_3
                (Widget|RemovefromParent _array_element_3)))))))
    (else
      (Variables|Default|SetcurrPlanetFocused 0)
      (Timeline|Timeline_0 PlayFromStart))))

(event EventBeginPlay
  (bind _allplanets (Variables|Default|GetAllPlanets))
  ;[1 1 1] Setting Orbit Center
  (for _array_element _allplanets
    (bind _output_get (Variables|Default|SetSumPositions (+ (Transformation|GetActorLocation _array_element) (Variables|Default|GetSumPositions))))
    (bind _asbp_planet (Utilities|Casting|CastToBP_Planet _array_element))
    (EventDispatchers|BindEventtoOnPlanetFocus _asbp_planet (EventDispatchers|CreateEvent :!event Custom|OnPlanetFocus)))
  (Variables|Default|SetOrbitCenter (/ _output_get (Utilities|Array|Length _allplanets)))
  (Variables|Default|SetPlayerCtrl (Game|GetPlayerController 0))
  (bind _output_get_2 (Variables|Default|SetPlayer (Game|Player|GetPlayerPawn 0)))
  (Variables|Default|SetStartPlayerPos (Transformation|GetActorLocation _output_get_2))
  (Variables|Default|SetStartPlayerRot "-33.000000,90.000000,0.000000"))

(event EventTick
  (params (DeltaSeconds :type Float%20%28single-precision%29))
  ;[1 1 1] Orbit Planets
  (if (Variables|Default|GetisOrbiting)
    (CallFunction|OrbitPlanets DeltaSeconds)))

(fn ConstructionScript)

(fn GetNewPosX
  (params (currX :type Float%20%28double-precision%29) (currAngle :type Float%20%28double-precision%29))
  (return (+ currX (* (Variables|Default|GetOrbitRadius) (Math|Trig|Cos(Degrees) currAngle)))))

(fn GetNewPosY
  (params (currY :type Float%20%28double-precision%29) (currAngle :type Float%20%28double-precision%29))
  (return (+ currY (* (Variables|Default|GetOrbitRadius) (Math|Trig|Sin(Degrees) currAngle)))))

(fn OrbitPlanets
  (params (deltaTime :type Float%20%28double-precision%29))
  (bind _orbitcenter (Variables|Default|GetOrbitCenter))
  (bind (_x _y) (Math|Vector|BreakVector _orbitcenter))
  ;[1 1 1] Set Orbit Positions For Planets
  (for (_array_element _array_index) (Variables|Default|GetAllPlanets)
    (|SetBy-RefVar (Utilities|Array|Get(acopy) (Variables|Default|GetInitialAngles) _array_index) (+ (Utilities|Array|Get(acopy) (Variables|Default|GetInitialAngles) _array_index) (+ (Variables|Default|GetOrbitSpeed) deltaTime)))
    (bind _output_get (Variables|Default|SetCurrentAngle (+ (Utilities|Array|Get(acopy) (Variables|Default|GetInitialAngles) _array_index) (+ (Variables|Default|GetOrbitSpeed) deltaTime))))
    (bind _newy (CallFunction|GetNewPosY _y _output_get))
    (bind _newx (CallFunction|GetNewPosX _x _output_get))
    (Class|KismetMathLibrary|VectorSet (Variables|Default|GetNewPosition) _newx _newy (.Z (Math|Vector|BreakVector (Transformation|GetActorLocation _array_element))))
    (bind _output_get_2 (Variables|Default|SetNewPosition (Variables|Default|GetNewPosition)))
    (Transformation|SetActorLocation _array_element _output_get_2 false false)))

(fn SetVectorsforPlanetView
  (params (ViewDistance :type Float%20%28double-precision%29))
  (bind _player (Variables|Default|GetPlayer))
  (bind _currplanetfocused (Variables|Default|GetcurrPlanetFocused))
  (bind _returnvalue (Transformation|GetActorLocation _player))
  (bind _returnvalue_2 (Transformation|GetActorLocation _currplanetfocused))
  (bind _returnvalue_3 (Math|Rotator|FindLookatRotation _returnvalue _returnvalue_2))
  (Variables|Default|SetCurrPlayerPos _returnvalue)
  (Variables|Default|SetNewPlayerRot _returnvalue_3)
  (Variables|Default|SetNewPlayerPos (- _returnvalue_2 (* (Math|Vector|GetForwardVector _returnvalue_3) ViewDistance))))

(fn SetVectorsforSystemView
  (Variables|Default|SetCurrPlayerPos (Transformation|GetActorLocation (Variables|Default|GetPlayer)))
  (Variables|Default|SetNewPlayerPos (Variables|Default|GetStartPlayerPos))
  (Variables|Default|SetNewPlayerRot (Variables|Default|GetStartPlayerRot)))

(fn MovePlayertoNewView
  (params (DistanceAlpha :type Float%20%28double-precision%29) (RotationAlpha :type Float%20%28double-precision%29))
  (bind _player (Variables|Default|GetPlayer))
  (Transformation|SetActorLocation _player (Math|Vector|Lerp(Vector) (Variables|Default|GetCurrPlayerPos) (Variables|Default|GetNewPlayerPos) DistanceAlpha) false false)
  (Transformation|SetActorRotation _player (Math|Rotator|Lerp(Rotator) (Transformation|GetActorRotation _player) (Variables|Default|GetNewPlayerRot) RotationAlpha)))