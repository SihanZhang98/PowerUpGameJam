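; Outcome manager actor that decides and presents a Best, Good or Bad result for the focused planet.
; CalculateOutcome takes the planet from BP_SystemManager and counts SelectedElements matching its data table row to grade FireOutcome.
; Best requires top fire and character grades; otherwise CharacterOutcome alone separates Good from Bad.
; The result text is stored on the planet and shown through DisplayOutcome with an attached Niagara effect and W_ShowOutcome widget.
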(event Custom|CalculateOutcome
  (bind _outactors (Actor|GetAllActorsOfClass "/Game/SolarSystem/BP_SystemManager.BP_SystemManager_C"))
  (bind _output_get (Variables|Default|SetCurr%20Planet%20Focused (Variables|/Game/SolarSystem/BP_SystemManager.BP_SystemManager_C|GetcurrPlanetFocused (Utilities|Array|Get(acopy) _outactors))))
  (Variables|/Game/SolarSystem/BP_Planet.BP_Planet_C|SethasOutcome _output_get true)
  (bind _returnvalue (Utilities|GetDataTableRow (.datatable (Variables|/Game/SolarSystem/BP_Planet.BP_Planet_C|GetPlanetData (Variables|/Game/SolarSystem/BP_SystemManager.BP_SystemManager_C|GetcurrPlanetFocused (Utilities|Array|Get(acopy) _outactors)))) (.rowname (Variables|/Game/SolarSystem/BP_Planet.BP_Planet_C|GetPlanetData (Variables|/Game/SolarSystem/BP_SystemManager.BP_SystemManager_C|GetcurrPlanetFocused (Utilities|Array|Get(acopy) _outactors)))))
    (:then
      (Utilities|FlowControl|Sequence
        (:then_0
          (for _array_element (Variables|Default|GetSelectedElements)
            (for _array_element_2 (.ElementsNeeded (Utilities|Struct|BreakStruct_Planet _returnvalue))
              (if (Utilities|Enum|Equal(Enum) _array_element_2 _array_element)
                (Math|Integer|IncrementInt (Variables|Default|GetCorrectElementAmount)))))
          (Development|PrintString (Utilities|String|ToString(Integer) (Variables|Default|GetCorrectElementAmount)))
          (switch int (Variables|Default|GetCorrectElementAmount)
            (:0
              (Variables|Default|SetFireOutcome "NewEnumerator2"))
            (:1
              (Variables|Default|SetFireOutcome "NewEnumerator1" :!label _label))
            (:2
              (goto _label))
            (:3
              (Variables|Default|SetFireOutcome "NewEnumerator0"))))
        (:then_1
          (if (and (Utilities|Enum|Equal(Enum) (Variables|Default|GetFireOutcome) "NewEnumerator0") (Utilities|Enum|Equal(Enum) (Variables|Default|GetCharacterOutcome) "NewEnumerator0"))
            (Variables|Default|SetFinalOutcome "NewEnumerator0")
            (bind _output_get_2 (Variables|Default|SetCurrOutcomeText (.BestOutcomeText (Utilities|Struct|BreakStruct_Planet _returnvalue))))
            (CallFunction|DisplayOutcome "/Game/Outcomes/PS_PlanetBest.PS_PlanetBest" _output_get_2)
            (Variables|/Game/SolarSystem/BP_Planet.BP_Planet_C|SetcurrOutcomeTxt (Variables|Default|GetCurr%20Planet%20Focused) _output_get_2)
            (elif (or (Utilities|Enum|Equal(Enum) (Variables|Default|GetCharacterOutcome) "NewEnumerator0") (Utilities|Enum|Equal(Enum) (Variables|Default|GetCharacterOutcome) "NewEnumerator1"))
              (Variables|Default|SetFinalOutcome "NewEnumerator1")
              (bind _output_get_3 (Variables|Default|SetCurrOutcomeText (.GoodOutcomeText (Utilities|Struct|BreakStruct_Planet _returnvalue))))
              (CallFunction|DisplayOutcome "/Game/Outcomes/PS_PlanetGood.PS_PlanetGood" _output_get_3)
              (Variables|/Game/SolarSystem/BP_Planet.BP_Planet_C|SetcurrOutcomeTxt (Variables|Default|GetCurr%20Planet%20Focused) _output_get_3)
              (else
                (Variables|Default|SetFinalOutcome "NewEnumerator2")
                (bind _output_get_4 (Variables|Default|SetCurrOutcomeText (.BadOutcomeText (Utilities|Struct|BreakStruct_Planet _returnvalue))))
                (CallFunction|DisplayOutcome "/Game/Outcomes/PS_PlanetBad.PS_PlanetBad" _output_get_4)
                (Variables|/Game/SolarSystem/BP_Planet.BP_Planet_C|SetcurrOutcomeTxt (Variables|Default|GetCurr%20Planet%20Focused) _output_get_4)))))))))

(event EventBeginPlay)

(event Collision|EventActorBeginOverlap
  (params (OtherActor :type Actor%20Object%20Reference)))

(fn ConstructionScript)

(fn DisplayOutcome
  (params (currEffect :type Niagara%20System%20Object%20Reference) (outcomeText :type Text))
  (Niagara|SpawnSystemAttached currEffect (Variables|/Game/SolarSystem/BP_Planet.BP_Planet_C|GetPlanet1-repackaged_Planet_1_001 (Variables|Default|GetCurr%20Planet%20Focused)) "None" "0, 0, 0" "0, 0, 0" "SnapToTarget" false)
  (bind _returnvalue (UserInterface|CreateWidget "/Game/Outcomes/W_ShowOutcome.W_ShowOutcome_C" (Game|GetPlayerController 0)))
  (UserInterface|Viewport|AddtoViewport _returnvalue 0)
  (Rendering|Components|TextRender|SetText (Variables|/Game/Outcomes/W_ShowOutcome.W_ShowOutcome_C|GetOutcomeText _returnvalue) outcomeText))