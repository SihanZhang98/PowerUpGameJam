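; Player pawn for a point-and-click scene where the player talks to planet characters with the mouse.
; BeginPlay shows the cursor, enables mouse click and hover events, and sets a fixed pawn rotation.
; A left click traces under the cursor, calls TalkMessage on a hit BP_PlanetCharacter and records it as talked to.
; A fire button widget appears whenever the unique talked-to count is divisible by three; title screen logic is disconnected.
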(event EventBeginPlay
  (bind _returnvalue (Game|GetPlayerController 0))
  (Variables|/Script/Engine.PlayerController|SetbShowMouseCursor _returnvalue true)
  (Variables|/Script/Engine.PlayerController|SetbEnableClickEvents _returnvalue true)
  (Variables|/Script/Engine.PlayerController|SetbEnableMouseOverEvents _returnvalue true)
  (Transformation|SetActorRotation (Game|Player|GetPlayerPawn 0) "327.000000,90.000000,0.000000"))

(event Input|MouseEvents|LeftMouseButton
  (params (Key :type Key%20Structure :default "None"))
  (:Pressed
    (bind _asbp_planet_character (Utilities|Casting|CastToBP_PlanetCharacter (.hitactor (.HitResult (Game|Player|GetHitResultUnderCursorbyChannel (Game|GetPlayerController 0) "TraceTypeQuery1" true)))))
    (Development|PrintString "Hello")
    (Class|InterfaceTalk|Talk(Message) _asbp_planet_character)
    (Utilities|Array|AddUnique (Variables|Default|GetTalkedToCharacters) (.RowName (Utilities|Struct|BreakDataTableRowHandle (Variables|/Game/Blueprints/BP_PlanetCharacter.BP_PlanetCharacter_C|GetCharacterData _asbp_planet_character))))
    (if (== (Math|Integer|%(Integer) (Utilities|Array|Length (Variables|Default|GetTalkedToCharacters)) 3) 0)
      (bind _returnvalue (UserInterface|CreateWidget "/Game/SolarSystem/Widgets/UI_FireBtn.UI_FireBtn_C" (Game|GetPlayerController 0)))
      (UserInterface|Viewport|AddtoViewport _returnvalue 0))))

(fn ConstructionScript)