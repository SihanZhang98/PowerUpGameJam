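; BP_PlanetCharacter is a character that highlights on cursor hover and can show a dialogue UI.
; BeginPlay applies PersonMaterial to the mesh, and hover toggles its "Selected" material parameter while IsViewFocused is true.
; The Talk event looks up the character's data table row, creates W_ShowCharacter, fills in its image and dialogues, then adds it to the viewport.
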(event OnBeginCursorOver(CharacterMesh)
  (params (TouchedComponent :type Primitive%20Component%20Object%20Reference))
  (if (Variables|Default|GetisViewFocused)
    (Rendering|Material|SetScalarParameterValueonMaterials (Variables|Default|GetCharacterMesh) "Selected" 1.0)))

(event OnEndCursorOver(CharacterMesh)
  (params (TouchedComponent :type Primitive%20Component%20Object%20Reference))
  (if (Variables|Default|GetisViewFocused)
    (Rendering|Material|SetScalarParameterValueonMaterials (Variables|Default|GetCharacterMesh) "Selected" 0.0)))

(event EventBeginPlay
  (Rendering|Material|SetMaterial (Variables|Default|GetCharacterMesh) 0 (Variables|Default|GetPersonMaterial)))

(event EventTalk
  (bind _characterdata (Variables|Default|GetCharacterData))
  (bind (_datatable _rowname) (Utilities|Struct|BreakDataTableRowHandle _characterdata))
  ;[1 1 1] get character data
  (bind _returnvalue (Utilities|GetDataTableRow _datatable _rowname)
    (:then
      ;[1 1 1] create widget
      (bind _returnvalue_2 (UserInterface|CreateWidget "/Game/SolarSystem/Widgets/W_ShowCharacter.W_ShowCharacter_C" (Game|GetPlayerController 0)))
      (Variables|Default|SetCharacterUI _returnvalue_2)
      ;[1 1 1] set character image and text based on character data
      (Appearance|SetBrushfromTexture (Variables|/Game/SolarSystem/Widgets/W_ShowCharacter.W_ShowCharacter_C|GetCharacterImage (Variables|Default|GetCharacterUI)) (.Image (Utilities|Struct|BreakStruct_Chracter _returnvalue)) false)
      (Variables|/Game/SolarSystem/Widgets/W_ShowCharacter.W_ShowCharacter_C|SetDialogues (Variables|Default|GetCharacterUI) (.Dialogues (Utilities|Struct|BreakStruct_Chracter _returnvalue)))
      (UserInterface|Viewport|AddtoViewport (Variables|Default|GetCharacterUI) 0))))

(fn ConstructionScript)